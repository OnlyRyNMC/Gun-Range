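; A wall-style button Blueprint that the player presses with Interact to swing a door open or closed.
; Box overlaps with SMG_Character_BP toggle input and a Gate, limiting presses to players in range.
; The Button Animation macro uses two timelines to push the mesh in and back out between transforms cached at BeginPlay.
; Its output drives a FlipFlop that plays or reverses DoorTimeline, lerping door yaw between closed and open angles.
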(event `self.ReceiveBeginPlay`
  (bind (_returnvalue_location _returnvalue_rotation _returnvalue_scale) (`KismetMathLibrary.BreakTransform` (`SceneComponent.GetRelativeTransform` (`self.StaticMesh`))))
  (set `self.OutPos` (`KismetMathLibrary.MakeTransform` _returnvalue_location _returnvalue_rotation _returnvalue_scale)) ; Out = not pressed
  (set `self.InPos` (`KismetMathLibrary.MakeTransform` (- _returnvalue_location (0.0 20.0 0.0)) _returnvalue_rotation _returnvalue_scale)) ; In = buttons pressed in
  (`self.EnableInput` (`GameplayStatics.GetPlayerController` 0)) ; Enables player to actually click the button
)

(event `InputAction|Interact`
  (params (Key :type "Key Structure"))
  ;[1 1 1] Pushing the button
  (:`Pressed`
    (`/Engine/EditorBlueprintResources/StandardMacros.Gate` true :!label _label
      (:`Exit`
        (bind (_direction _button_in) (`Timeline|Button In` :!via `PlayFromStart`) ; Timeline so that the button in only takes .5 seconds
          (:`Update`
            (`SceneComponent.K2_SetRelativeTransform` (`self.StaticMesh`) (`KismetMathLibrary.TLerp` (`self.OutPos`) (`self.InPos`) _button_in) false false))
          (:`Finished`
            (bind (_direction_2 _button_in_2) (`Timeline|Button Out` :!via `ReverseFromEnd`) ; Using reverse from end legit means play backwards (so button is going out)
              (:`Update`
                (`SceneComponent.K2_SetRelativeTransform` (`self.StaticMesh`) (`KismetMathLibrary.TLerp` (`self.OutPos`) (`self.InPos`) _button_in_2) false false))
              (:`Finished`
                _))
            (`/Engine/EditorBlueprintResources/StandardMacros.FlipFlop`
              (:`A`
                (bind (_direction_3 _door_track) (`Timeline|Door Timeline` :!label _label_2)
                  (:`Update`
                    (`SceneComponent.K2_SetRelativeRotation` (`self.Door`) (`KismetMathLibrary.MakeRotator` 0.0 0.0 (`KismetMathLibrary.Lerp` (`self.Door Close Angle`) (`self.Door Open Angle`) _door_track)) false false))))
              (:`B`
                (goto _label_2 :!via `Reverse`)))))))))

(event `self.Box.OnComponentBeginOverlap`
  (params (OverlappedComponent :type "PrimitiveComponent Object Reference") (OtherActor :type "Actor Object Reference") (OtherComp :type "PrimitiveComponent Object Reference") (OtherBodyIndex :type Integer) (bFromSweep :type Boolean) (SweepResult :type "HitResult Structure (by ref)"))
  ;[1 1 1] Pushing the button
  (cast `/Game/Blueprints/Weapons/SMG/SMG_Character_BP` OtherActor)
  (`self.EnableInput` (`GameplayStatics.GetPlayerController` 0))
  (goto _label :!via `Open`))

(event `self.Box.OnComponentEndOverlap`
  (params (OverlappedComponent :type "PrimitiveComponent Object Reference") (OtherActor :type "Actor Object Reference") (OtherComp :type "PrimitiveComponent Object Reference") (OtherBodyIndex :type Integer))
  ;[1 1 1] Pushing the button
  (cast `/Game/Blueprints/Weapons/SMG/SMG_Character_BP` OtherActor)
  (`self.DisableInput` (`GameplayStatics.GetPlayerController` 0))
  (goto _label :!via `Close`))

(fn `UserConstructionScript`)